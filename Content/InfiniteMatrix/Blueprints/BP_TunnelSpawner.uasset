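; Spawner actor that builds a chain of BP_Tunnel segments and populates them with health packs and enemies.
; On BeginPlay it clears existing tunnels, packs and enemies, then spawns an initial run starting at the player pawn, each next segment at the newest one's SpawnPoint.
; Each tunnel gets a spawner reference and randomized wall, with a coin-flip health pack.
; Enemies spawn only alongside packs, and their 80.0 chance check always passes.
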(event `self.ReceiveBeginPlay`
  (`self.SpawnInitialTunnels`))

(fn `SpawnInitialTunnels`
  (`|ExecutionSequence`
    (:`then_0`
      (bind _outactors (`GameplayStatics.GetAllActorsOfClass` "/Game/InfiniteMatrix/Blueprints/BP_Tunnel.BP_Tunnel_C"))
      (for _array_element _outactors
        (`self.K2_DestroyActor` _array_element))
      (bind _outactors_2 (`GameplayStatics.GetAllActorsOfClass` "/Game/InfiniteMatrix/Blueprints/BP_HealthPack.BP_HealthPack_C"))
      (for _array_element_2 _outactors_2
        (`self.K2_DestroyActor` _array_element_2))
      (bind _outactors_3 (`GameplayStatics.GetAllActorsOfClass` "/Game/InfiniteMatrix/Blueprints/BP_Enemy.BP_Enemy_C"))
      (for _array_element_3 _outactors_3
        (`self.K2_DestroyActor` _array_element_3)))
    (:`then_1`
      (for _ (range 4)
        (`/Engine/EditorBlueprintResources/StandardMacros.IsValid` (`self.Newest Tunnel`)
          (:`Is Valid`
            (`self.SpawnTunnelAtSpawnPoint`))
          (:`Is Not Valid`
            (`self.SpawnTunnel` (`self.K2_GetActorLocation` (`GameplayStatics.GetPlayerPawn` 0)))))))))

(fn `SpawnTunnel`
  (params (SpawnLocation :type "Vector Structure"))
  (bind _returnvalue (`|SpawnActorFromClass` "/Game/InfiniteMatrix/Blueprints/BP_Tunnel.BP_Tunnel_C" (`KismetMathLibrary.MakeTransform` SpawnLocation) "Undefined" "OverrideRootScale" null null))
  (bind _output_get (set `self.Newest Tunnel` _returnvalue))
  (set `/Game/InfiniteMatrix/Blueprints/BP_Tunnel.TunnelSpawner` self _output_get)
  (`/Game/InfiniteMatrix/Blueprints/BP_Tunnel.RandomizeWall` _output_get)
  (if (< (`KismetMathLibrary.RandomFloat`) 0.5)
    (bind _returnvalue_2 (`|SpawnActorFromClass` "/Game/InfiniteMatrix/Blueprints/BP_HealthPack.BP_HealthPack_C" (`KismetMathLibrary.MakeTransform` (+ SpawnLocation (`KismetMathLibrary.MakeVector` 1000.0 (`KismetMathLibrary.RandomFloatInRange` -300.0 300.0) (`KismetMathLibrary.RandomFloatInRange` -300.0 300.0)))) "Undefined" "OverrideRootScale" null null))
    (set `/Game/InfiniteMatrix/Blueprints/BP_Tunnel.HealthPack` _returnvalue_2 _returnvalue)
    (set `/Game/InfiniteMatrix/Blueprints/BP_HealthPack.ParentTunnel` _returnvalue _returnvalue_2)
    (if (< (`KismetMathLibrary.RandomFloat`) 80.0)
      (bind _returnvalue_3 (`|SpawnActorFromClass` "/Game/InfiniteMatrix/Blueprints/BP_Enemy.BP_Enemy_C" (`KismetMathLibrary.MakeTransform` (+ SpawnLocation (`KismetMathLibrary.MakeVector` 2200.0 (`KismetMathLibrary.RandomFloatInRange` -300.0 300.0) (`KismetMathLibrary.RandomFloatInRange` -300.0 300.0)))) "Undefined" "OverrideRootScale" null null))
      (set `/Game/InfiniteMatrix/Blueprints/BP_Tunnel.Enemy` _returnvalue_3 _returnvalue))))

(fn `SpawnTunnelAtSpawnPoint`
  (`self.SpawnTunnel` (`SceneComponent.K2_GetComponentLocation` (`/Game/InfiniteMatrix/Blueprints/BP_Tunnel.SpawnPoint` (`self.Newest Tunnel`)))))

(fn `UserConstructionScript`)