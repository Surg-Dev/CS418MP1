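; BP_Projectile is a short-lived projectile that travels along world X and gets faster as the player's score rises.
; Each Tick it applies a swept world offset from ForwardSpeed plus a multiple of the Score on the first BP_Player found at BeginPlay.
; A timer set at BeginPlay calls DProj to destroy it after under a second, and the graph has no active overlap or hit handling.
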(event `self.ReceiveBeginPlay`
  (bind _outactors (`GameplayStatics.GetAllActorsOfClass` "/Game/InfiniteMatrix/Blueprints/BP_Player.BP_Player_C"))
  (`KismetSystemLibrary.K2_SetTimer` null "DProj" 0.75))

(event `self.ReceiveTick`
  (params (DeltaSeconds :type "Float (single-precision)"))
  (`self.K2_AddActorWorldOffset` (`KismetMathLibrary.MakeVector` (* DeltaSeconds (+ (`self.ForwardSpeed`) (* 50.0 (`/Game/InfiniteMatrix/Blueprints/BP_Player.Score` (`|GetArrayItem` (stale `self.ReceiveBeginPlay` _outactors))))))) true))

(fn `DProj`
  (`self.K2_DestroyActor`))

(fn `UserConstructionScript`)