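; BP_Enemy is an enemy actor whose skeleton head mesh reacts to overlaps with the player or projectiles.
; Touching the player destroys the enemy, costs one health, removes a heart widget, shakes the camera, and triggers death and the restart display at zero health.
; A projectile hit destroys both actors and increments the score on the first BP_Player found in the world.
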(event `self.SM_SkeletonHead.OnComponentBeginOverlap`
  (params (OverlappedComponent :type "PrimitiveComponent Object Reference") (OtherActor :type "Actor Object Reference") (OtherComp :type "PrimitiveComponent Object Reference") (OtherBodyIndex :type Integer) (bFromSweep :type Boolean) (SweepResult :type "HitResult Structure (by ref)"))
  (bind _asbp_player (cast `/Game/InfiniteMatrix/Blueprints/BP_Player` OtherActor)
    (:`then`
      (`self.K2_DestroyActor`)
      (bind _result (`/Engine/EditorBlueprintResources/StandardMacros.DecrementInt` (`/Game/InfiniteMatrix/Blueprints/BP_Player.Health` _asbp_player))
        (:`  `
          (`Widget.RemoveFromParent` (`|GetArrayItem` (`/Game/InfiniteMatrix/Blueprints/BP_Player.HeartWidget` _asbp_player) _result))
          (`PlayerCameraManager.StartCameraShake` :`self` (`PlayerController.PlayerCameraManager` (`Pawn.GetLocalViewingPlayerController` _asbp_player)) :`ShakeClass` "/Game/InfiniteMatrix/Blueprints/CameraShake.CameraShake_C")
          (if (== _result 0)
            (set `/Game/InfiniteMatrix/Blueprints/BP_Player.isDead` true _asbp_player)
            (`/Game/InfiniteMatrix/Blueprints/BP_Player.DisplayRestart` _asbp_player)))))
    (:`CastFailed`
      (bind _asbp_projectile (cast `/Game/InfiniteMatrix/Blueprints/BP_Projectile` OtherActor))
      (`self.K2_DestroyActor` _asbp_projectile)
      (`self.K2_DestroyActor`)
      (bind _outactors (`GameplayStatics.GetAllActorsOfClass` "/Game/InfiniteMatrix/Blueprints/BP_Player.BP_Player_C"))
      (`/Engine/EditorBlueprintResources/StandardMacros.IncrementInt` (`/Game/InfiniteMatrix/Blueprints/BP_Player.Score` (`|GetArrayItem` _outactors))))))

(fn `UserConstructionScript`)